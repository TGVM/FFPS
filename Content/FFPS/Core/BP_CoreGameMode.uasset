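; Game mode for a two-team match with elemental characters, handling team assignment, spawning and scoring.
; BeginPlay sorts PlayerStarts by tag, while PostLogin waits for that setup, then alternates players between gamestate teams.
; A looping timer calls each controller to add its input map once MaxPlayers have joined.
; PickCharacter spawns and possesses the chosen class at the player's team slot, and IncreaseScore updates team points through the gamestate.
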(event Custom|IncreaseScore
  (params (Team :type Integer))
  (bind _core_gamestate (Variables|Default|GetCore%20Gamestate))
  (switch int Team
    (:1
      (Math|Integer|IncrementInt (Variables|/Game/FFPS/Core/BP_CoreGamestate.BP_CoreGamestate_C|GetPointsTeamOne _core_gamestate)
        (:%20%20
          (Default|ForceRepPointsTeam1 _core_gamestate))))
    (:2
      (Math|Integer|IncrementInt (Variables|/Game/FFPS/Core/BP_CoreGamestate.BP_CoreGamestate_C|GetPointsTeamTwo _core_gamestate)
        (:%20%20
          (Default|ForceRepPointsTeam2 _core_gamestate))))))

(event Custom|AllPlayersOn
  (if (== (Utilities|Array|Length (Variables|/Script/Engine.GameStateBase|GetPlayerArray (Game|GetGameState))) (Variables|Default|GetMaxPlayers))
    (Utilities|Time|ClearandInvalidateTimerbyHandle (Variables|Default|GetAllPlayersOn_Timer))
    (for _array_element (Variables|Default|GetPlayerControllerArray)
      (Default|OCAddInputMap _array_element))))

(event EventBeginPlay
  (Variables|Default|SetMaxPlayers (Math|Conversions|ToInteger(Byte) (Class|GameplayStatics|ParseOption (Variables|Default|GetOptionsString) "MaxPlayers")))
  (bind _asbp_core_gamestate (Utilities|Casting|CastToBP_CoreGamestate (Game|GetGameState)))
  (Variables|Default|SetCore%20Gamestate _asbp_core_gamestate)
  (bind _outactors (Actor|GetAllActorsOfClass "/Script/Engine.PlayerStart"))
  (for _array_element _outactors
    (if (Actor|ActorHasTag _array_element "Team1")
      (Utilities|Array|Add (Variables|Default|GetPlayerStartsTeam1) _array_element)
      (else
        (Utilities|Array|Add (Variables|Default|GetPlayerStartsTeam2) _array_element))))
  (Variables|Default|SetHasBegun true)
  (bind _returnvalue (Utilities|Time|SetTimerbyEvent (delegate Custom|AllPlayersOn) 1.0 true))
  (Variables|Default|SetAllPlayersOn_Timer _returnvalue))

(event EventTick
  (params (DeltaSeconds :type Float%20%28single-precision%29)))

(event EventPostLogin
  (params (NewPlayer :type Player%20Controller%20Object%20Reference))
  (bind _core_gamestate (Variables|Default|GetCore%20Gamestate))
  (if (Variables|Default|GetHasBegun) :!label _label
    (bind _asbp_main_player_controller (Utilities|Casting|CastToBP_MainPlayerController NewPlayer))
    (Utilities|Array|Add (Variables|Default|GetPlayerControllerArray) _asbp_main_player_controller)
    (Utilities|FlowControl|FlipFlop
      (:A
        (bind _returnvalue (Utilities|Array|Add (Variables|/Game/FFPS/Core/BP_CoreGamestate.BP_CoreGamestate_C|GetTeam1 _core_gamestate) _asbp_main_player_controller))
        (Variables|/Game/FFPS/MainCharacter/BP_MainPlayerController.BP_MainPlayerController_C|SetTeamPosition _asbp_main_player_controller _returnvalue)
        (Variables|/Game/FFPS/MainCharacter/BP_MainPlayerController.BP_MainPlayerController_C|SetTeam _asbp_main_player_controller 1))
      (:B
        (bind _returnvalue_2 (Utilities|Array|Add (Variables|/Game/FFPS/Core/BP_CoreGamestate.BP_CoreGamestate_C|GetTeam2 _core_gamestate) _asbp_main_player_controller))
        (Variables|/Game/FFPS/MainCharacter/BP_MainPlayerController.BP_MainPlayerController_C|SetTeamPosition _asbp_main_player_controller _returnvalue_2)
        (Variables|/Game/FFPS/MainCharacter/BP_MainPlayerController.BP_MainPlayerController_C|SetTeam _asbp_main_player_controller 2)))
    (else
      (Utilities|FlowControl|Delay 0.5)
      (goto _label))))

(fn ConstructionScript)

(fn SpawnCharacterOfClass
  (params (PlayerController :type BP%20Main%20Player%20Controller%20Object%20Reference) (Class :type Actor%20Class%20Reference) (team :type Integer) (TeamPosition :type Integer))
  (switch int team
    (:1
      (LocalVariables|SetSelected%20Spawn (Transformation|GetActorTransform (Utilities|Array|Get(acopy) (Variables|Default|GetPlayerStartsTeam1) TeamPosition))))
    (:2
      (LocalVariables|SetSelected%20Spawn (Transformation|GetActorTransform (Utilities|Array|Get(acopy) (Variables|Default|GetPlayerStartsTeam2) TeamPosition)))))
  (bind _returnvalue (Game|SpawnActorfromClass Class (LocalVariables|GetSelected%20Spawn) "AlwaysSpawn" "MultiplyWithRoot" PlayerController 0))
  (bind _asbp_base_character (Utilities|Casting|CastToBP_BaseCharacter _returnvalue))
  (Pawn|Possess PlayerController _asbp_base_character))

(fn PickCharacter
  (params (CharacterType :type String) (PlayerController :type BP%20Main%20Player%20Controller%20Object%20Reference))
  (switch string CharacterType
    (:Default
      (LocalVariables|SetCharacterClass "/Game/FFPS/MainCharacter/BP_BaseCharacter.BP_BaseCharacter_C"))
    (:Air
      (LocalVariables|SetCharacterClass "/Game/FFPS/MainCharacter/BP_AirCharacterPawn.BP_AirCharacterPawn_C"))
    (:Earth
      (LocalVariables|SetCharacterClass "/Game/FFPS/MainCharacter/BP_EarthCharacterPawn.BP_EarthCharacterPawn_C"))
    (:Fire
      (LocalVariables|SetCharacterClass "/Game/FFPS/MainCharacter/BP_FireCharacterPawn.BP_FireCharacterPawn_C"))
    (:Water
      (LocalVariables|SetCharacterClass "/Game/FFPS/MainCharacter/BP_WaterCharacterPawn.BP_WaterCharacterPawn_C")))
  (CallFunction|SpawnCharacterOfClass PlayerController (LocalVariables|GetCharacterClass) (Variables|/Game/FFPS/MainCharacter/BP_MainPlayerController.BP_MainPlayerController_C|GetTeam PlayerController) (Variables|/Game/FFPS/MainCharacter/BP_MainPlayerController.BP_MainPlayerController_C|GetTeamPosition PlayerController))
  (Default|OCRemoveBeginUI PlayerController))