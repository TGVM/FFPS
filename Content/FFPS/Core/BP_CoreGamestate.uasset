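; Game state Blueprint for the FFPS core that holds replicated point totals for two teams and keeps the score display current.
; Each team's OnRep function calls a matching ForceRep function, which can also serve as a direct refresh.
; That function casts player controller 0 to BP_MainPlayerController and, if its ScoreUI is valid, pushes the points and team number through UpdateScore.
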(event EventBeginPlay)

(event EventTick
  (params (DeltaSeconds :type Float%20%28single-precision%29)))

(fn ConstructionScript)

(fn OnRepPointsTeamOne
  (CallFunction|ForceRepPointsTeam1))

(fn OnRepPointsTeamTwo
  (CallFunction|ForceRepPointsTeam2))

(fn ForceRepPointsTeam1
  (bind _asbp_main_player_controller (Utilities|Casting|CastToBP_MainPlayerController (Game|GetPlayerController 0)))
  (Utilities|IsValid (Variables|/Game/FFPS/MainCharacter/BP_MainPlayerController.BP_MainPlayerController_C|GetScoreUI _asbp_main_player_controller)
    (:Is%20Valid
      (Default|UpdateScore (Variables|/Game/FFPS/MainCharacter/BP_MainPlayerController.BP_MainPlayerController_C|GetScoreUI _asbp_main_player_controller) (Variables|Default|GetPointsTeamOne) 1))))

(fn ForceRepPointsTeam2
  (bind _asbp_main_player_controller (Utilities|Casting|CastToBP_MainPlayerController (Game|GetPlayerController 0)))
  (Utilities|IsValid (Variables|/Game/FFPS/MainCharacter/BP_MainPlayerController.BP_MainPlayerController_C|GetScoreUI _asbp_main_player_controller)
    (:Is%20Valid
      (Default|UpdateScore (Variables|/Game/FFPS/MainCharacter/BP_MainPlayerController.BP_MainPlayerController_C|GetScoreUI _asbp_main_player_controller) (Variables|Default|GetPointsTeamTwo) 2))))