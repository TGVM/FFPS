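; BP_MainPlayerController is the player controller that routes Enhanced Input to the possessed BP_BaseCharacter.
; Movement input passes straight through, while look input applies scaled yaw on the controller and sends scaled, inverted pitch to the character's LookUpDown.
; Both shoot press and release call SVShoot with the action value.
; OC_AddInputMap registers the IMC_PlayerCommands mapping context on the local player's input subsystem.
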(event Custom|OC_AddInputMap
  (Input|AddMappingContext (PlayerController|LocalPlayerSubsystems|GetEnhancedInputLocalPlayerSubsystem) "/Game/FFPS/MainCharacter/IMC_PlayerCommands.IMC_PlayerCommands" 0 "(bIgnoreAllPressedKeysUntilRelease=True,bForceImmediately=False,bNotifyUserSettings=False)"))

(event Input|EnhancedActionEvents|EnhancedInputActionIA_Movement
  (params (ActionValue :type Vector%202D%20Structure) (ElapsedSeconds :type Float%20%28double-precision%29) (TriggeredSeconds :type Float%20%28double-precision%29) (InputAction :type Input%20Action%20Object%20Reference :default "/Game/FFPS/MainCharacter/IA_Movement.IA_Movement"))
  (bind _asbp_base_character (Utilities|Casting|CastToBP_BaseCharacter (Pawn|GetControlledPawn)))
  (Default|Movement _asbp_base_character ActionValue))

(event Input|EnhancedActionEvents|EnhancedInputActionIA_Look
  (params (ActionValue :type Vector%202D%20Structure) (ElapsedSeconds :type Float%20%28double-precision%29) (TriggeredSeconds :type Float%20%28double-precision%29) (InputAction :type Input%20Action%20Object%20Reference :default "/Game/FFPS/MainCharacter/IA_Look.IA_Look"))
  (Class|PlayerController|AddYawInput (* (Variables|Default|GetHorizontalSensibility) (.x ActionValue)))
  (bind _asbp_base_character (Utilities|Casting|CastToBP_BaseCharacter (Pawn|GetControlledPawn)))
  (Default|LookUpDown _asbp_base_character (* (* (Variables|Default|GetVerticalSensibility) (.y ActionValue)) -1.0)))

(event Input|EnhancedActionEvents|EnhancedInputActionIA_Shoot
  (params (ActionValue :type Boolean) (ElapsedSeconds :type Float%20%28double-precision%29) (TriggeredSeconds :type Float%20%28double-precision%29) (InputAction :type Input%20Action%20Object%20Reference :default "/Game/FFPS/MainCharacter/IA_Shoot.IA_Shoot"))
  (:Started
    (bind _asbp_base_character (Utilities|Casting|CastToBP_BaseCharacter (Pawn|GetControlledPawn) :!label _label))
    (Default|SVShoot _asbp_base_character ActionValue))
  (:Completed
    (goto _label)))

(fn ConstructionScript)